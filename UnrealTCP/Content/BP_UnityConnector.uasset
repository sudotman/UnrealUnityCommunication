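; Test connector that links Unreal to a Unity server by IP and port, connecting shortly after BeginPlay.
; Debug keys reconnect, disconnect or send a greeting as bytes, and connection events print to screen.
; Received messages are read as strings, and their first four characters select a Cube or Sphere branch that spawns at a random location.
; Only the sphere branch sets an actor class; byte and transform parsing nodes are unwired.
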(event Custom|onDisconnected
  (params (ConnectionId :type Integer))
  (Development|PrintString "disconnected from server" true true "(R=1.000000,G=0.000000,B=0.206878,A=1.000000)"))

(event Custom|onConnected
  (params (ConnectionId :type Integer))
  (Development|PrintString (Utilities|String|Append (Utilities|String|ToString(Integer) ConnectionId) " is the connection id")))

(event Custom|recievedMessage
  (params (ConnectionId :type Integer) (Message :type Array%20of%20Bytes))
  (Development|PrintString "recieved message from unity" true true "(R=1.000000,G=0.435228,B=0.284806,A=1.000000)")
  (bind _returnvalue (Class|TcpSocketConnection|MessageReadString Message 35))
  (Development|PrintString _returnvalue true true "(R=0.000000,G=1.000000,B=0.322387,A=1.000000)" 5.0)
  (switch string (Utilities|String|GetSubstring _returnvalue 0 4)
    (:Cube
      (Game|SpawnActorfromClass "/Game/testCube.testCube_C" (Math|Transform|MakeTransform (Math|Vector|MakeVector (Math|Random|RandomFloatinRange -7e+02 7e+02) (Math|Random|RandomFloatinRange -7e+02 7e+02) (Math|Random|RandomFloatinRange 1e+02 3e+02))) "Undefined" 0 0))
    (:Sphe
      (Game|SpawnActorfromClass "/Game/testSphere.testSphere_C" (Math|Transform|MakeTransform (Math|Vector|MakeVector (Math|Random|RandomFloatinRange -7e+02 7e+02) (Math|Random|RandomFloatinRange -7e+02 7e+02) (Math|Random|RandomFloatinRange 1e+02 3e+02))) "Undefined" 0 0))))

(event EventBeginPlay
  (Development|PrintString "Connecting now..")
  (Utilities|FlowControl|Delay 1.0)
  (bind _connectionid (Class|TcpSocketConnection|Connect (Variables|Default|GetIP%20Address) (Variables|Default|GetPort) (delegate Custom|onDisconnected) (delegate Custom|onConnected) (delegate Custom|recievedMessage))))

(event EventTick
  (params (DeltaSeconds :type Float%20%28single-precision%29)))

(event Input|KeyboardEvents|1
  (params (Key :type Key%20Structure :default "None"))
  (:Pressed
    (Development|PrintString "Sending message now" true true "(R=0.000000,G=0.660000,B=1.000000,A=1.000000)" 4.0)
    (bind _returnvalue (Class|TcpSocketConnection|SendData (stale EventBeginPlay _connectionid) (Class|TcpSocketConnection|ToBytes(String) "hi from unreal")))
    (Development|PrintString (Utilities|String|ToString(Boolean) _returnvalue))))

(event Input|KeyboardEvents|4
  (params (Key :type Key%20Structure :default "None"))
  (:Pressed
    (Development|PrintString "disconnecting")
    (Class|TcpSocketConnection|Disconnect (stale EventBeginPlay _connectionid))))

(event Input|KeyboardEvents|5
  (params (Key :type Key%20Structure :default "None"))
  (:Pressed
    (bind _connectionid (Class|TcpSocketConnection|Connect (Variables|Default|GetIP%20Address) (Variables|Default|GetPort) (delegate Custom|onDisconnected) (delegate Custom|onConnected) (delegate Custom|recievedMessage)))))

(fn ConstructionScript)